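; BP_White is an enemy monster Character that takes damage, reacts and dies.
; AnyDamage reduces Health and stores the instigator's pawn as Attacker, then plays a hit montage and snaps rotation toward it.
; At zero Health or below it plays a death montage and destroys itself after a short delay.
; Combat functions manage state and movement flags and play combo montages from WeaponDatas, while WeaponAttach is empty.
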(event Game|Damage|EventAnyDamage
  (params (Damage :type Float%20%28single-precision%29) (DamageType :type Damage%20Type%20Object%20Reference) (InstigatedBy :type Controller%20Object%20Reference) (DamageCauser :type Actor%20Object%20Reference))
  (|TakeDamage InstigatedBy Damage DamageCauser)
  (|HitReaction)
  (|CheckDead))

(fn ConstructionScript)

(fn PlayComboMontage
  (bind _weapondatas (Variables|Attack|GetWeaponDatas))
  (bind _combocount (Variables|Attack|GetComboCount))
  (bind _output (Utilities|Array|Get(acopy) _weapondatas _combocount))
  (Animation|PlayAnimMontage (.animmontage _output) (.playrate _output) (.startsection _output))
  (Variables|Default|SetCanMove (.canmove _output)))

(fn GetCombatType
  (return (Variables|Default|GetCombatType)))

(fn Hitted
  (Variables|Default|SetStateType "NewEnumerator0")
  (return false))

(fn IsStateAttacking
  (return (Utilities|Enum|Equal(Enum) (Variables|Default|GetStateType) "NewEnumerator2")))

(fn IsStateIdling
  (return (Utilities|Enum|Equal(Enum) (Variables|Default|GetStateType) "NewEnumerator0")))

(fn SetCanMove
  (params (CanMove :type Boolean))
  (Variables|Default|SetCanMove CanMove)
  (return false))

(fn SetCurrentState
  (params (WeaponPose :type EWeaponPose%20Enum :default "NewEnumerator1") (StateType :type EStateType%20Enum :default "NewEnumerator0"))
  (Variables|Default|SetWeaponPose WeaponPose)
  (Variables|Default|SetStateType StateType)
  (return))

(fn SetStateAttacking
  (Variables|Default|SetStateType "NewEnumerator2")
  (return false))

(fn SetStateIdling
  (Variables|Default|SetStateType "NewEnumerator0")
  (return false))

(fn WeaponAttach)

(fn WeaponEquipped
  (if (Utilities|Enum|Equal(Enum) (Variables|Default|GetStateType) "NewEnumerator1")
    (return false)))