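; Player character with camera-relative movement, walk and jump input, and automatic ledge hanging with climb up or drop.
; Every tick, downward and forward sphere traces find the ledge height and wall normal; a ledge near pelvis height triggers Hang.
; Hang switches to Flying, holds the climb montage at zero rate and aligns the capsule to the wall.
; X launches a ragdoll and quits after a delay; the sword spawn is unwired.
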(event EventTick
  (params (DeltaSeconds :type Float%20%28single-precision%29))
  (CallFunction|HeightTrace)
  (CallFunction|ForwardTrace))

(fn ConstructionScript)

(fn ForwardTrace
  (bind _returnvalue (Transformation|GetActorLocation))
  (bind _outhit (Collision|SphereTraceByChannel _returnvalue (+ _returnvalue (* (Transformation|GetActorForwardVector) 1.5e+02)) 1e+01 "TraceTypeQuery3" false 0 "None"))
  (Variables|Default|SetWallNormal (.Normal (Collision|BreakHitResult _outhit)))
  (Variables|Default|SetWallLocation (.Location (Collision|BreakHitResult _outhit))))

(fn HeightTrace
  (bind _returnvalue (Transformation|GetActorLocation))
  (bind _returnvalue_2 (Transformation|GetActorForwardVector))
  (bind _charactermovement (Variables|Character|GetCharacterMovement))
  (bind _returnvalue_3 (* _returnvalue_2 75.0))
  (bind _returnvalue_4 (+ _returnvalue "0, 0,500.000000" _returnvalue_3))
  (bind (_outhit _returnvalue_5) (Collision|SphereTraceByChannel _returnvalue_4 (- _returnvalue_4 "0, 0,500.000000") 1e+01 "TraceTypeQuery3" false 0 "None"))
  (if _returnvalue_5
    (Variables|Default|SetHeightLocation (.Location (Collision|BreakHitResult _outhit)))
    (if (Math|Float|InRange(Float) (- (.z (Transformation|GetSocketLocation (Variables|Character|GetMesh) "pelvisSocket")) (.Z (Math|Vector|BreakVector (.Location (Collision|BreakHitResult _outhit))))) -5e+01 0.0)
      (if (not (Variables|Default|GetIsClimbing))
        (Pawn|Components|CharacterMovement|SetMovementMode _charactermovement "MOVE_Flying" 0)
        (Components|Movement|StopMovementImmediately _charactermovement)
        (CallFunction|Hang)))))

(event Input|ActionEvents|InputActionWalking
  (params (Key :type Key%20Structure :default "None"))
  (bind _charactermovement (Variables|Character|GetCharacterMovement))
  (:Pressed
    (Variables|/Script/Engine.CharacterMovementComponent|SetMaxWalkSpeed _charactermovement 4e+02))
  (:Released
    (Variables|/Script/Engine.CharacterMovementComponent|SetMaxWalkSpeed _charactermovement 6e+02)))

(event Input|ActionEvents|InputActionJumping
  (params (Key :type Key%20Structure :default "None"))
  (:Pressed
    (if (Variables|Default|GetCanMove)
      (Character|Jump)))
  (:Released
    (Character|StopJumping)))

(event Input|AxisEvents|InputAxisMoveForward
  (params (AxisValue :type Float%20%28single-precision%29))
  (if (not (Variables|Default|GetIsClimbing))
    (if (Variables|Default|GetCanMove)
      (Pawn|Input|AddMovementInput (Math|Vector|GetForwardVector (Math|Rotator|MakeRotator 0.0 0.0 (.yaw (Pawn|GetControlRotation :!class /Script/Engine.Pawn)))) AxisValue false))))

(event Input|AxisEvents|InputAxisMoveRight
  (params (AxisValue :type Float%20%28single-precision%29))
  (if (not (Variables|Default|GetIsClimbing))
    (if (Variables|Default|GetCanMove)
      (Pawn|Input|AddMovementInput (Math|Vector|GetRightVector (Math|Rotator|MakeRotator 0.0 0.0 (.yaw (Pawn|GetControlRotation :!class /Script/Engine.Pawn)))) AxisValue false))))

(event Input|AxisEvents|InputAxisHorizontalLook
  (params (AxisValue :type Float%20%28single-precision%29))
  (Pawn|Input|AddControllerYawInput AxisValue))

(event Input|AxisEvents|InputAxisVerticalLook
  (params (AxisValue :type Float%20%28single-precision%29))
  (Pawn|Input|AddControllerPitchInput AxisValue))

(event Custom|Hang
  (bind _wallnormal (Variables|Default|GetWallNormal))
  (bind _walllocation (Variables|Default|GetWallLocation))
  (bind _returnvalue (* _wallnormal 21.0))
  (bind _returnvalue_2 (+ _returnvalue _walllocation))
  ;[1 1 1] Hanging
  (Animation|Montage|PlayMontage (Variables|Character|GetMesh) "/Game/Character/Animations/Climb/Hang_to_Crouch_fixed_Montage.Hang_to_Crouch_fixed_Montage" 0.0
    (:then
      (Variables|Default|SetIsClimbing true)
      (Components|MoveComponentTo (Variables|Collision|GetCapsuleComponent) (Math|Vector|MakeVector (.x _returnvalue_2) (.y _returnvalue_2) (- (.z (Variables|Default|GetHeightLocation)) 88.0)) (Math|Rotator|MakeRotfromX (* _wallnormal -1.0)) true true 0.2 false))))

(event Custom|Climb%20Up
  (Animation|Montage|PlayMontage (Variables|Character|GetMesh) "/Game/Character/Animations/Climb/Hang_to_Crouch_fixed_Montage.Hang_to_Crouch_fixed_Montage"
    (:OnNotifyBegin
      (Variables|Default|SetIsClimbing false)
      (Pawn|Components|CharacterMovement|SetMovementMode (Variables|Character|GetCharacterMovement) "MOVE_Walking" 0)
      (CallFunction|FinishedClimbing))))

(event Custom|Climb%20Down
  (Variables|Default|SetIsClimbing false)
  (Pawn|Components|CharacterMovement|SetMovementMode (Variables|Character|GetCharacterMovement) "MOVE_Falling" 0)
  (Animation|StopAnimMontage "/Game/Character/Animations/Climb/Hang_to_Crouch_fixed_Montage.Hang_to_Crouch_fixed_Montage"))

(event Custom|FinishedClimbing
  (Utilities|FlowControl|DoOnce false) ; enters at Reset
)

(event Input|ActionEvents|InputActionClimbUP
  (params (Key :type Key%20Structure :default "None"))
  (:Pressed
    (if (Variables|Default|GetIsClimbing)
      (Utilities|FlowControl|DoOnce false
        (:Completed
          (CallFunction|ClimbUp))))))

(event Input|ActionEvents|InputActionClimbDown
  (params (Key :type Key%20Structure :default "None"))
  (:Pressed
    (if (Variables|Default|GetIsClimbing)
      (CallFunction|ClimbDown))))

(event Custom|MakeRagdoll
  (bind _mesh (Variables|Character|GetMesh))
  (Collision|SetCollisionEnabled (Variables|Collision|GetCapsuleComponent) "NoCollision")
  (Variables|/Script/Engine.SpringArmComponent|SetbDoCollisionTest (Variables|Default|GetSpringArm) false)
  (Variables|/Script/Engine.SkeletalMeshComponent|SetGlobalAnimRateScale (Variables|Character|GetMesh) 0.0)
  (Physics|SetSimulatePhysics (Variables|Character|GetMesh) true)
  (Collision|SetCollisionEnabled _mesh "QueryAndPhysics")
  (Physics|AddForce _mesh "0, 0,500000.000000" "None" false)
  (Utilities|FlowControl|Delay 3.0)
  (Development|ExecuteConsoleCommand "Quit" (Game|GetPlayerController 0)))

(event Input|KeyboardEvents|X
  (params (Key :type Key%20Structure :default "None"))
  (:Pressed
    (CallFunction|MakeRagdoll)))

(event EventBeginPlay)