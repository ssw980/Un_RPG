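; Base melee weapon Blueprint that plays combo attack montages on its owning Character.
; BeginPlay gathers data table rows matching its weapon type as ordered combo steps, each setting montage, play rate, section and movement permission.
; Attack starts the combo or buffers input while CanCombo is open; PlayNextCombo advances buffered steps and EndAttack resets state.
; SendDamage filters already-hit actors, StartCombo and EndCombo are empty, and hit-stop effects are disconnected.
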(event Custom|PlayNextCombo
  (if (Variables|Default|GetSucceedCombo)
    (Variables|Default|SetSucceedCombo false)
    (Math|Integer|IncrementInt (Variables|Default|GetComboCount)
      (:%20%20
        (CallFunction|PlayComboMontage)
        (Variables|Default|SetLastCombo (== (Variables|Default|GetComboCount) (- (Utilities|Array|Length (Variables|Default|GetWeaponData)) 1)))))))

(event Custom|DamageEffect)

(event EventBeginPlay
  (|CallParentFunction)
  (bind _outrownames (DataTable|GetDataTableRowNames (Variables|Default|GetDataTable)))
  (for _array_element _outrownames
    (bind _returnvalue (Utilities|GetDataTableRow (Variables|Default|GetDataTable) _array_element)
      (:then
        (if (== (.Type (Utilities|Struct|BreakFMeleeData _returnvalue)) (Variables|Default|GetWeaponType))
          (Utilities|Array|Add (Variables|Default|GetWeaponData) _returnvalue))))))

(event EventTick
  (params (DeltaSeconds :type Float%20%28single-precision%29)))

(event EventAttack
  (|CallParentFunction)
  (if (Variables|Default|GetCanCombo)
    (Variables|Default|SetCanCombo false)
    (Variables|Default|SetSucceedCombo true)
    (else
      (CallFunction|PlayComboMontage)
      (CallFunction|StartCombo))))

(event EventEndAttack
  (|CallParentFunction)
  (CallFunction|SetStateIdling)
  (Variables|Default|SetComboCount 0)
  (CallFunction|SetCanMove true)
  (Variables|Default|SetSucceedCombo false)
  (Variables|Default|SetLastCombo false)
  (CallFunction|EndCombo))

(fn ConstructionScript
  (|CallParentFunction))

(fn PlayComboMontage
  (bind _weapondata (Variables|Default|GetWeaponData))
  (bind _combocount (Variables|Default|GetComboCount))
  (bind _output (Utilities|Array|Get(acopy) _weapondata _combocount))
  (bind _ascharacter (Utilities|Casting|CastToCharacter (Components|GetOwner)))
  (Animation|PlayAnimMontage _ascharacter (.animmontage _output) (.playrate _output) (.startsection _output))
  (CallFunction|SetCanMove (.canmove _output))
  (return))

(fn StartCombo)

(fn SendDamage
  (params (OtherActor :type Actor%20Object%20Reference) (Damage :type Float%20%28single-precision%29))
  (bind _array_element (Utilities|Array|ForEachLoopwithBreak (Variables|Default|GetHittedActors) :!label _label)
    (:LoopBody
      (if (== _array_element OtherActor)
        (LocalVariables|SetEverHittedActor true)
        (goto _label Break)))
    (:Completed
      (if (not (LocalVariables|GetEverHittedActor))
        (Utilities|Array|Add (Variables|Default|GetHittedActors) OtherActor)
        (bind _result (|CallParentFunction OtherActor Damage))
        (Utilities|Casting|CastToCharacter OtherActor)
        (if _result
          (return _result))))))

(fn EndCombo)